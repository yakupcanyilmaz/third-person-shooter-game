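; Player controller for a shooter that handles match-flow UI and pawn input locking.
; Events show countdown, info and end-game widgets, freeze or unfreeze the controlled pawn's input, and open the multiplayer main menu level.
; Pressing Enter casts to ShooterGameModeBP and calls its Countdown.
; The end-game event clears all widgets before passing the win and tie result to its widget, and the TargetScore RepNotify is empty.
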(event `self.ReceiveBeginPlay`)

(event `ShowCountdown`
  (bind _returnvalue (`|CreateWidget` "/Game/_Game/HUD/CountdownWidgetBP.CountdownWidgetBP_C"))
  (`UserWidget.AddToViewport` _returnvalue 0))

(event `UnFreeze`
  (`self.EnableInput` (`self.K2_GetPawn`) self))

(event `Key|Enter`
  (params (Key :type "Key Structure"))
  (:`Pressed`
    (bind _asshooter_game_mode_bp (cast `/Game/_Game/GameMode/ShooterGameModeBP` (`GameplayStatics.GetGameMode`)))
    (`/Game/_Game/GameMode/ShooterGameModeBP.Countdown` _asshooter_game_mode_bp)))

(event `ShowInfo`
  (bind _returnvalue (`|CreateWidget` "/Game/_Game/HUD/InfoWidgetBP.InfoWidgetBP_C"))
  (`UserWidget.AddToViewport` _returnvalue 0))

(event `Freeze`
  (`self.DisableInput` (`self.K2_GetPawn`) self))

(event `ShowEndGameWidget`
  (params (Won :type Boolean) (Tie :type Boolean))
  (`WidgetLayoutLibrary.RemoveAllWidgets`)
  (bind _returnvalue (`|CreateWidget` "/Game/_Game/HUD/EndGameWidgetBP.EndGameWidgetBP_C" null Won Tie))
  (`UserWidget.AddToViewport` _returnvalue 0))

(event `BackToMainMenu`
  (`GameplayStatics.OpenLevel` "MultiMainMenuLevel"))

(fn `OnRep_TargetScore`)

(fn `UserConstructionScript`)