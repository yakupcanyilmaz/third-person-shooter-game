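; Bottle target Blueprint that displays a score number popup on screen when its show-score event fires.
; The event relays through server-named and client-named events, which creates a score number widget at the bottle's projected screen position for player controller 0.
; It also prints a "HIT" debug string and passes no score value to the widget.
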(event `self.OnShowTargetScore`
  (`self.ShowTargetScoreOnServer`))

(event `ShowTargetScoreOnServer`
  (`self.ShowTargetScoreOnClient`))

(event `ShowTargetScoreOnClient`
  (bind _returnvalue (`|CreateWidget` "/Game/_Game/HUD/ScoreNumberWidgetBP.ScoreNumberWidgetBP_C"))
  (`UserWidget.AddToViewport` _returnvalue 0)
  (`UserWidget.SetPositionInViewport` _returnvalue (`GameplayStatics.ProjectWorldToScreen` (`GameplayStatics.GetPlayerController` 0) (`self.K2_GetActorLocation`)) true)
  (`KismetSystemLibrary.PrintString` "HIT"))

(fn `UserConstructionScript`)