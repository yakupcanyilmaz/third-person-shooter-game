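; HUD Blueprint that draws a dynamic four-piece crosshair at screen center for the player's ShooterCharacterBP.
; It caches the character on BeginPlay, and DrawHUD retries that lookup whenever the reference is invalid.
; Each DrawHUD offsets the top, bottom, left and right textures outward by the character's spread multiplier times a maximum spread.
; The crosshair is hidden while the character is sprinting and moving.
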(event `self.ReceiveBeginPlay`
  (`/Engine/EditorBlueprintResources/StandardMacros.IsValid` (`self.ShooterCharacter`) :!label _label
    (:`Is Not Valid`
      (bind _asshooter_character_bp (cast `/Game/_Game/Character/ShooterCharacterBP` (`GameplayStatics.GetPlayerPawn` 0)))
      (set `self.ShooterCharacter` _asshooter_character_bp))))

(event `self.ReceiveDrawHUD`
  (params (SizeX :type Integer) (SizeY :type Integer))
  (bind _shootercharacter (`self.ShooterCharacter`))
  (bind (_x _y) (`KismetMathLibrary.BreakVector2D` (`self.CrosshairLocation`)))
  (bind (_x_2 _y_2) (`KismetMathLibrary.BreakVector2D` (`self.CrosshairBaseCenter`)))
  (bind (_x_3 _y_3) (`KismetMathLibrary.BreakVector2D` (`self.CrosshairBaseCenter`)))
  (bind (_x_4 _y_4) (`KismetMathLibrary.BreakVector2D` (`self.CrosshairBaseCenter`)))
  (bind (_x_5 _y_5) (`KismetMathLibrary.BreakVector2D` (`self.CrosshairBaseCenter`)))
  (bind (_x_6 _y_6) (`KismetMathLibrary.BreakVector2D` (`self.ScreenCenter`)))
  (`/Engine/EditorBlueprintResources/StandardMacros.IsValid` (`self.ShooterCharacter`)
    (:`Is Valid`
      (set `self.ScreenCenter` (`KismetMathLibrary.MakeVector2D` (`KismetMathLibrary.Conv_IntToDouble` (/ SizeX 2)) (`KismetMathLibrary.Conv_IntToDouble` (/ SizeY 2))))
      (set `self.CrosshairLocation` (`KismetMathLibrary.MakeVector2D` _x_6 _y_6))
      (`/Engine/EditorBlueprintResources/StandardMacros.IsValid` _shootercharacter
        (:`Is Valid`
          _)
        (:`Is Not Valid`
          (cast `/Game/_Game/Character/ShooterCharacterBP` (`GameplayStatics.GetPlayerPawn` 0))
          (set `self.ShooterCharacter` null)))
      (set `self.CrosshairSpreadMultiplier` (`ShooterCharacter.GetCrosshairSpreadMultiplier` _shootercharacter))
      (set `self.CrosshairBaseCenter` (`KismetMathLibrary.MakeVector2D` (- _x (`self.CrosshairHalfWidth`)) (- _y (`self.CrosshairHalfHeight`))))
      (if (or (not (`ShooterCharacter.bSprinting` _shootercharacter)) (== (`self.GetVelocity` _shootercharacter) (0.0 0.0 0.0)))
        (`self.DrawTexture` "/Game/_Game/FX/Textures/Crosshairs/Crosshair_Quad_9_Bottom.Crosshair_Quad_9_Bottom" _x_3 (+ _y_3 (* (`self.CrosshairSpreadMultiplier`) (`self.CrosshairSpreadMax`))) 64.0 64.0 0.0 0.0 1.0 1.0)
        (`self.DrawTexture` "/Game/_Game/FX/Textures/Crosshairs/Crosshair_Quad_9_Top.Crosshair_Quad_9_Top" _x_4 (- _y_4 (* (`self.CrosshairSpreadMultiplier`) (`self.CrosshairSpreadMax`))) 64.0 64.0 0.0 0.0 1.0 1.0)
        (`self.DrawTexture` "/Game/_Game/FX/Textures/Crosshairs/Crosshair_Quad_9_Left.Crosshair_Quad_9_Left" (- _x_5 (* (`self.CrosshairSpreadMultiplier`) (`self.CrosshairSpreadMax`))) _y_5 64.0 64.0 0.0 0.0 1.0 1.0)
        (`self.DrawTexture` "/Game/_Game/FX/Textures/Crosshairs/Crosshair_Quad_9_Right.Crosshair_Quad_9_Right" (+ (* (`self.CrosshairSpreadMultiplier`) (`self.CrosshairSpreadMax`)) _x_2) _y_2 64.0 64.0 0.0 0.0 1.0 1.0)))
    (:`Is Not Valid`
      (goto _label))))

(fn `UserConstructionScript`)